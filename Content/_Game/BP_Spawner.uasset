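; Spawner that builds a maze-like map out of BP_Cube actors on BeginPlay.
; SpawnCubes lays out a centred square grid, giving each cube a running index and storing it in BPCubes.
; DestroyCubes opens cells at odd row and column positions, leaving a wall lattice.
; GenerateMap, defined outside this file, then returns coordinates that are flattened into array indices to remove further cubes.
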(event `self.ReceiveBeginPlay`
  (set `self.Size` 51)
  (`self.Spawn Cubes` (`self.Size`))
  (`self.Destroy Cubes` (`self.Size`))
  (bind (_y _x) (`self.GenerateMap` (`self.Size`)))
  (for (_ _array_index) _y
    (`self.K2_DestroyActor` (`|GetArrayItem` (`self.BP_Cubes`) (+ (`|GetArrayItem` _y _array_index) (* (`|GetArrayItem` _x _array_index) (`self.Size`)))))))

(fn `Destroy Cubes`
  (params (Size :type Integer))
  (locals (NewLocalVar_0 :type Integer))
  (set `local.NewLocalVar_0` Size)
  (for _array_element (`self.BP_Cubes`)
    (bind _idx (`/Game/_Game/BP_Cube.Idx` _array_element))
    (if (not (or (== (mod (mod _idx (`local.NewLocalVar_0`)) 2) 0) (== (mod (/ _idx (`local.NewLocalVar_0`)) 2) 0)))
      (`self.K2_DestroyActor` _array_element))))

(fn `Spawn Cubes`
  (params (size :type Integer))
  (locals (NewLocalVar :type Integer))
  (set `local.NewLocalVar` size)
  (set `self.LocX` (`KismetMathLibrary.Conv_IntToDouble` (* (+ (/ (`local.NewLocalVar`) 2) 1) 1000)))
  (for _ (range 1 (+ (`local.NewLocalVar`) 1))
    (set `self.LocX` (- (`self.LocX`) 1000.0))
    (set `self.LocY` (`KismetMathLibrary.Conv_IntToDouble` (* (/ (`local.NewLocalVar`) 2) 1000)))
    (for _ (range 1 (+ (`local.NewLocalVar`) 1))
      (bind _returnvalue (`|SpawnActorFromClass` "/Game/_Game/BP_Cube.BP_Cube_C" (`KismetMathLibrary.Conv_VectorToTransform` (`KismetMathLibrary.MakeVector` (`self.LocX`) (`self.LocY`) 500.0)) "AdjustIfPossibleButAlwaysSpawn" "OverrideRootScale" null (`self.Idx`) null))
      (`KismetArrayLibrary.Array_Add` (`self.BP_Cubes`) _returnvalue)
      (set `self.LocY` (- (`self.LocY`) 1000.0))
      (`/Engine/EditorBlueprintResources/StandardMacros.IncrementInt` (`self.Idx`)))))

(fn `UserConstructionScript`)